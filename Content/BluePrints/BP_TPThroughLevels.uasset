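; Teleporter actor that sends the player to a random level picked from its LevelsList.
; It stays inactive until the referenced Spawner fires its level-created event, which enables teleporting.
; When the player character's capsule then overlaps the Trigger, it plays a WB_Fade widget animation and opens the chosen level by object reference after a short delay.
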(event `self.ReceiveBeginPlay`
  (add `EnemySpawner.OnLevelCreared` (`self.Spawner`) (delegate `MakeTeleportWorking`)))

(event `MakeTeleportWorking`
  (set `self.CanTeleport` true))

(event `self.Trigger.OnComponentBeginOverlap`
  (params (OverlappedComponent :type "PrimitiveComponent Object Reference") (OtherActor :type "Actor Object Reference") (OtherComp :type "PrimitiveComponent Object Reference") (OtherBodyIndex :type Integer) (bFromSweep :type Boolean) (SweepResult :type "HitResult Structure (by ref)"))
  (if (`self.CanTeleport`)
    (cast `/Game/ThirdPerson/Blueprints/BP_ThirdPersonCharacter` OtherActor)
    (if (== OtherComp (`Character.CapsuleComponent` (`GameplayStatics.GetPlayerCharacter` 0)))
      (bind _returnvalue (`|CreateWidget` "/Game/UI/WB_Fade.WB_Fade_C"))
      (`UserWidget.AddToViewport` _returnvalue 0)
      (`/Game/UI/WB_Fade.FadeAnim` _returnvalue)
      (`KismetSystemLibrary.Delay` 0.5)
      (`GameplayStatics.OpenLevelBySoftObjectPtr` (`self.GetRandomLevel`)))))

(fn `GetRandomLevel`
  (returns (RandomLevel :type "World Soft Object Reference"))
  (locals (NewLocalVar :type "World Soft Object Reference"))
  (return (`KismetArrayLibrary.Array_Random` (`self.LevelsList`))))

(fn `UserConstructionScript`)