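; BP_EnemyAI is an enemy that detects the player, deals damage to them and takes health effects itself.
; PawnSensing sets the hasSeenPlayer Blackboard key when it sees the third-person character.
; Helper checks test line of sight with a debug-drawn visibility trace, height difference, and distance against a padded AttackDistance.
; Damage sends GE_TestDamage to the player as a health effect message, while incoming effects pass to HealthManagerComponent.
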(event `self.PawnSensing.OnSeePawn`
  (params (Pawn :type "Pawn Object Reference"))
  (cast `/Game/ThirdPerson/Blueprints/BP_ThirdPersonCharacter` Pawn)
  (`BlackboardComponent.SetValueAsBool` (`AIBlueprintHelperLibrary.GetBlackboard` (`AIBlueprintHelperLibrary.GetAIController` self)) "hasSeenPlayer" true))

(event `GiveDamageToPlayer`
  (message `IHealthHaving.ApplyHealthEffect` (`GameplayStatics.GetPlayerCharacter` 0) "/Game/GameplayEffects/HealthEffects/GE_TestDamage.GE_TestDamage_C"))

(event `self.ApplyHealthEffect`
  (params (Effect :type "GameplayEffect Class Reference"))
  (message `IHealthHaving.ApplyHealthEffect` (`self.HealthManagerComponent`) Effect))

(fn `Check Distance to Player`
  (returns (result :type Boolean))
  (return (<= (`KismetMathLibrary.Vector_Distance` (`self.K2_GetActorLocation` (`GameplayStatics.GetPlayerCharacter` 0)) (`self.K2_GetActorLocation` self)) (+ (`self.attackDistance`) 100.0))))

(fn `CheckForWalls`
  (returns (Result :type Boolean))
  (bind _outhit (`KismetSystemLibrary.LineTraceSingle` :`Start` (`self.K2_GetActorLocation` self) :`End` (`self.K2_GetActorLocation` (`GameplayStatics.GetPlayerCharacter` 0)) :`TraceChannel` "TraceTypeQuery1" :`DrawDebugType` "ForDuration"))
  (return (not (`GameplayStatics.BreakHitResult` _outhit))))

(fn `CompareAIAndPlayerHight`
  (returns (Result :type Boolean))
  (return (<= (`KismetMathLibrary.Abs` (- (.z (`self.K2_GetActorLocation` (`GameplayStatics.GetPlayerCharacter` 0))) (.z (`self.K2_GetActorLocation` self)))) 103.0)))

(fn `UserConstructionScript`)